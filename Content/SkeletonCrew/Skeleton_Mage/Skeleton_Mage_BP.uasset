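; Skeleton mage enemy that repositions and fires projectiles at the first DummyPlayerActor.
; After its spawn montage, it loops: the FindArcherSpot EQS query picks a spot, AIMoveTo walks there, then it turns, plays the attack montage and spawns Projectile1.
; Stun pauses movement for a hit montage, then re-enters the loop at the last queried spot.
; Die runs once, setting IsDying to block further actions, then plays death montage and effect before destroying the actor.
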(event EventBeginPlay
  (Animation|Montage|PlayMontage (Variables|Character|GetMesh) "/Game/SkeletonCrew/Skeleton_Mage/Animations/Skeleton_Mage_Spawn_Montage.Skeleton_Mage_Spawn_Montage"
    (:OnCompleted
      (bind _returnvalue (AI|EQS|RunEQSQuery "/Game/AI/FindArcherSpot.FindArcherSpot" self "RandomBest25Pct" :!label _label))
      (Utilities|FlowControl|Delay 0.2)
      (bind (_resultlocations _returnvalue_2) (AI|EQS|GetQueryResultsasLocations _returnvalue))
      (if _returnvalue_2
        (AI|AIMoveTo self (Utilities|Array|Get(acopy) _resultlocations) 0 1e+01 false
          (:OnSuccess
            (if (not (Variables|Default|GetisDying))
              (bind _outactors (Actor|GetAllActorsOfClass "/Game/DummyPlayerActor.DummyPlayerActor_C"))
              (Transformation|SetActorRotation (Math|Rotator|MakeRotator 0.0 0.0 (.yaw (Math|Rotator|FindLookatRotation (Transformation|GetActorLocation) (Transformation|GetActorLocation (Utilities|Array|Get(acopy) _outactors))))))
              (Animation|Montage|PlayMontage (Variables|Character|GetMesh) "/Game/SkeletonCrew/Skeleton_Mage/Animations/Skeleton_Mage_Default_Attack_Montage.Skeleton_Mage_Default_Attack_Montage"
                (:then
                  (Components|Activation|Activate (Variables|Default|GetCrossbowFX) true)
                  (Utilities|FlowControl|Delay 0.9)
                  (if (not (Variables|Default|GetisDying))
                    (Game|SpawnActorfromClass "/Game/SkeletonCrew/Skeleton_Mage/Projectile1.Projectile1_C" (Math|Transform|MakeTransform (Transformation|GetSocketLocation (Variables|Character|GetMesh) "hand_lSocket") (Math|Rotator|MakeRotator 0.0 -5.0 (.yaw (Transformation|GetActorRotation))) "1.000000,1.000000,1.000000") "Undefined" "OverrideRootScale" 0 0)))
                (:OnCompleted
                  (goto _label)))))
          (:OnFail
            (goto _label)))
        (else
          (goto _label))))))

(event EventStun
  (bind _charactermovement (Variables|Character|GetCharacterMovement))
  (bind _isdying (Variables|Default|GetisDying))
  (Pawn|Components|CharacterMovement|SetMovementMode _charactermovement "MOVE_None" 0)
  (Animation|Montage|PlayMontage (Variables|Character|GetMesh) "/Game/SkeletonCrew/Skeleton_Mage/Animations/Skeleton_Mage_Hit_Front_Montage.Skeleton_Mage_Hit_Front_Montage"
    (:then
      (Utilities|FlowControl|Delay 1.0)
      (if (not _isdying)
        (Pawn|Components|CharacterMovement|SetMovementMode _charactermovement "MOVE_Walking" 0)
        (AI|AIMoveTo self (Utilities|Array|Get(acopy) (stale _resultlocations)) 0 1e+01 false :!label _label
          (:OnSuccess
            (if (not _isdying)
              (bind _outactors (Actor|GetAllActorsOfClass "/Game/DummyPlayerActor.DummyPlayerActor_C"))
              (Transformation|SetActorRotation (Math|Rotator|MakeRotator 0.0 0.0 (.yaw (Math|Rotator|FindLookatRotation (Transformation|GetActorLocation) (Transformation|GetActorLocation (Utilities|Array|Get(acopy) _outactors))))))
              (Animation|Montage|PlayMontage (Variables|Character|GetMesh) "/Game/SkeletonCrew/Skeleton_Mage/Animations/Skeleton_Mage_Default_Attack_Montage.Skeleton_Mage_Default_Attack_Montage"
                (:then
                  (Components|Activation|Activate (Variables|Default|GetCrossbowFX) true)
                  (Utilities|FlowControl|Delay 0.9)
                  (if (not (Variables|Default|GetisDying))
                    (Game|SpawnActorfromClass "/Game/SkeletonCrew/Skeleton_Mage/Projectile1.Projectile1_C" (Math|Transform|MakeTransform (Transformation|GetSocketLocation (Variables|Character|GetMesh) "hand_lSocket") (Math|Rotator|MakeRotator 0.0 -5.0 (.yaw (Transformation|GetActorRotation))) "1.000000,1.000000,1.000000") "Undefined" "OverrideRootScale" 0 0)))
                (:OnCompleted
                  (bind _returnvalue (AI|EQS|RunEQSQuery "/Game/AI/FindArcherSpot.FindArcherSpot" self "RandomBest25Pct" :!label _label_2))
                  (Utilities|FlowControl|Delay 0.2)
                  (bind (_resultlocations _returnvalue_2) (AI|EQS|GetQueryResultsasLocations _returnvalue))
                  (if _returnvalue_2
                    (goto _label)
                    (else
                      (goto _label_2)))))))
          (:OnFail
            (goto _label_2)))))))

(event EventDie
  (bind _mesh (Variables|Character|GetMesh))
  (Utilities|FlowControl|DoOnce false
    (:Completed
      (Audio|Components|Audio|Stop (Variables|Character|GetMesh))
      (Variables|Default|SetisDying true)
      (Pawn|Components|CharacterMovement|SetMovementMode (Variables|Character|GetCharacterMovement) "MOVE_None" 0)
      (Animation|Montage|PlayMontage (Variables|Character|GetMesh) "/Game/SkeletonCrew/Skeleton_Mage/Animations/Skeleton_Mage_Die_Montage.Skeleton_Mage_Die_Montage"
        (:then
          (Utilities|FlowControl|Delay 0.96)
          (Rendering|SetVisibility _mesh false false)
          (Collision|SetCollisionEnabled _mesh "NoCollision")
          (Components|Activation|Activate (Variables|Default|GetEnemyDeathEffect) false)
          (Utilities|FlowControl|Delay 2.0)
          (Actor|DestroyActor))))))

(fn ConstructionScript
  (Transformation|AttachComponentToComponent (Variables|Default|GetCrossbowFX) (Variables|Character|GetMesh) "hand_l" "SnapToTarget" "SnapToTarget" "SnapToTarget" true))